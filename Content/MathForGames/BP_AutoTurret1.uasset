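; Auto turret that rises when the player pawn is within detection range and lowers when out of range.
; In range, Tick yaws the actor toward the player, using the cross product's Z sign for turn direction and the dot product to confirm aim.
; When aligned, it spawns an impulse-launched projectile, then waits on a cooldown timer.
; Rotation scales with delta time; height moves a fixed step per tick.
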(event `self.ReceiveBeginPlay`
  ;[1 1 1] Turret Rotation
  (set `self.PlayerRef` (`GameplayStatics.GetPlayerPawn` 0)))

(event `self.ReceiveTick`
  (params (DeltaSeconds :type "Float (single-precision)"))
  (bind _returnvalue (`self.GetActorForwardVector`))
  (bind _playerref (`self.PlayerRef`))
  (bind _projectilespawner (`self.ProjectileSpawner`))
  (bind _z (.z (`SceneComponent.RelativeLocation` (`self.TurretBase`))))
  (bind _returnvalue_2 (- (`self.K2_GetActorLocation` _playerref) (`self.K2_GetActorLocation`)))
  (bind _returnvalue_3 (`KismetMathLibrary.Normal` _returnvalue_2))
  (bind (_returnvalue_x _returnvalue_y _returnvalue_z) (`KismetMathLibrary.BreakVector` (`KismetMathLibrary.Cross_VectorVector` _returnvalue _returnvalue_3)))
  ;[1 1 1] Turret Rotation
  (if (`KismetSystemLibrary.IsValid` _playerref)
    (`/Engine/EditorBlueprintResources/StandardMacros.CompareFloat` (`KismetMathLibrary.VSize` _returnvalue_2) (`self.DetectionRange`)
      (:`>`
        ;[1 1 1] Rise & Fall
        (`/Engine/EditorBlueprintResources/StandardMacros.CompareFloat` _z (`self.minHeight`)
          (:`>`
            (if true
              (`SceneComponent.K2_AddLocalOffset` (`self.TurretBase`) (0.0 0.0 -1.5) false false)))))
      (:`<`
        (`|ExecutionSequence`
          (:`then_0`
            (`/Engine/EditorBlueprintResources/StandardMacros.CompareFloat` _z (`self.maxHeight`)
              (:`<`
                (if true
                  (`SceneComponent.K2_AddLocalOffset` (`self.TurretBase`) (0.0 0.0 1.5) false false)))))
          (:`then_1`
            (if (> (`KismetMathLibrary.Dot_VectorVector` _returnvalue _returnvalue_3) 0.99)
              (if (`self.canShoot`)
                (bind _returnvalue_4 (`|SpawnActorFromClass` "/Game/MathForGames/BP_Projectile.BP_Projectile_C" (`SceneComponent.K2_GetComponentToWorld` _projectilespawner) "Undefined" "MultiplyWithRoot" null null))
                (`PrimitiveComponent.AddImpulse` (`/Game/MathForGames/BP_Projectile.Projectile` _returnvalue_4) (* (`SceneComponent.GetForwardVector` _projectilespawner) 200.0) "None" false)
                (set `self.canShoot` false)
                (`KismetSystemLibrary.K2_SetTimerDelegate` (delegate `ResetCanShoot`) (`self.ShootCooldown`)))
              (elif (> _returnvalue_z 0.0)
                (`self.K2_AddActorLocalRotation` (`KismetMathLibrary.MakeRotator` 0.0 0.0 (* (`GameplayStatics.GetWorldDeltaSeconds`) (`self.RotationSpeed`))))
                (else
                  (`self.K2_AddActorLocalRotation` (`KismetMathLibrary.MakeRotator` 0.0 0.0 (* (`GameplayStatics.GetWorldDeltaSeconds`) (`self.RotationSpeed`) -1.0))))))))))))

(event `ResetCanShoot`
  (set `self.canShoot` true))

(fn `UserConstructionScript`)