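; BP_PlayerKart is a player kart that drives forward and backward along its facing direction from the DriveForward input axis.
; The axis value, scaled by delta time, accumulates into Acceleration, which is clamped between negative and positive Speed and acts as velocity.
; That value offsets the actor along its forward vector without sweep or frame-time scaling, and is printed for debugging.
; It has no drag or steering.
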(event `InputAxis|DriveForward`
  (params (AxisValue :type "Float (single-precision)"))
  (bind _speed (`self.Speed`))
  (bind _output_get (set `self.Acceleration` (`KismetMathLibrary.FClamp` (+ (* AxisValue 3.0 (`GameplayStatics.GetWorldDeltaSeconds`)) (`self.Acceleration`)) (* _speed -1.0) _speed)))
  (`KismetSystemLibrary.PrintString` (`KismetStringLibrary.Conv_DoubleToString` _output_get))
  (`self.K2_AddActorWorldOffset` (* _output_get (`self.GetActorForwardVector`))))

(fn `UserConstructionScript`)