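; BP_PlayerSphere is a player sphere Blueprint that handles Fire input with a barrel recoil animation and cooldown.
; When the Fire axis reads 1 and no cooldown is active, it snaps the Barrel's target arm length short.
; A delay-driven loop then extends the arm in steps and clears the cooldown at full length.
; No projectile or damage logic is present in the graph.
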(event `InputAxis|Fire`
  (params (AxisValue :type "Float (single-precision)"))
  (bind _barrel (`self.Barrel`))
  (if (== AxisValue 1.0)
    (if (not (`self.IsFireOnCooldown`))
      (set `self.IsFireOnCooldown` true)
      (set `SpringArmComponent.TargetArmLength` 15.0 _barrel)
      (`KismetSystemLibrary.Delay` 0.2)
      (if (< (`SpringArmComponent.TargetArmLength` _barrel) 60.0) :!label _label
        (set `SpringArmComponent.TargetArmLength` (+ (`SpringArmComponent.TargetArmLength` (`self.Barrel`)) 5.0) _barrel)
        (`KismetSystemLibrary.Delay` 0.2)
        (goto _label)
        (else
          (set `self.IsFireOnCooldown` false))))))

(fn `UserConstructionScript`)