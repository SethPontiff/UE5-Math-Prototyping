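; BP_Projectile is a short-lived projectile actor that explodes on impact and pushes physics objects.
; It sets a lifespan on BeginPlay so that projectiles which hit nothing expire.
; On hit, it spawns an explosion emitter at the impact point and, if the struck component simulates physics, applies an impulse there along the projectile's forward vector, scaled by ImpulseStrength, before destroying itself.
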(event `self.ReceiveBeginPlay`
  (`self.SetLifeSpan` 3.0))

(event `self.ReceiveHit`
  (params (MyComp :type "PrimitiveComponent Object Reference") (Other :type "Actor Object Reference") (OtherComp :type "PrimitiveComponent Object Reference") (bSelfMoved :type Boolean) (HitLocation :type "Vector Structure") (HitNormal :type "Vector Structure") (NormalImpulse :type "Vector Structure") (Hit :type "HitResult Structure (by ref)"))
  (bind (_bblockinghit _binitialoverlap _time _distance _location) (`GameplayStatics.BreakHitResult` Hit))
  (`GameplayStatics.SpawnEmitterAtLocation` "/Game/StarterContent/Particles/P_Explosion.P_Explosion" _location)
  (if (`SceneComponent.IsSimulatingPhysics` OtherComp "None")
    (`PrimitiveComponent.AddImpulseAtLocation` OtherComp (* (`self.ImpulseStrength`) (`SceneComponent.GetForwardVector` (`self.Projectile`))) _location "None"))
  (`self.K2_DestroyActor`))

(fn `UserConstructionScript`)