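; Player-controlled physics tank that drives, jumps, aims and fires projectiles.
; TankForward applies both force and yaw angular velocity to CollisionBox, TankRight is empty, and a downward trace gates the jump impulse.
; Mouse input yaws the turret and pitches the clamped barrel, while holding Fire runs a looping timer that spawns impulse-launched BP_Projectiles.
; Camera input adjusts clamped FOV zoom and toggles a top-down camera.
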(event `InputAxis|TankForward`
  (params (AxisValue :type "Float (single-precision)"))
  ;[1 1 1] WASD Tank Movement
  (`PrimitiveComponent.AddForce` (`self.CollisionBox`) (* (* (`self.GetActorForwardVector`) (* AxisValue 300.0)) 3000.0) "None" false)
  (`PrimitiveComponent.SetPhysicsAngularVelocityInRadians` (`self.CollisionBox`) (`KismetMathLibrary.MakeVector` 0.0 0.0 (* (`GameplayStatics.GetWorldDeltaSeconds`) (* (`KismetMathLibrary.FClamp` (stale `InputAxis|TankRight` AxisValue) -1.0) 90.0))) false "None"))

(event `InputAxis|TankRight`
  (params (AxisValue :type "Float (single-precision)"))
  ;[1 1 1] WASD Tank Movement
)

(event `InputAction|Jump`
  (params (Key :type "Key Structure"))
  (:`Pressed`
    (bind (_outhits _returnvalue) (`KismetSystemLibrary.LineTraceMulti` (`self.K2_GetActorLocation`) (+ (`self.K2_GetActorLocation`) (0.0 0.0 -100.0)) "TraceTypeQuery1"))
    (if _returnvalue
      (`PrimitiveComponent.AddImpulse` (`self.CollisionBox`) (0.0 0.0 1000.0) "None" true))))

(event `InputAxis|MouseTurn`
  (params (AxisValue :type "Float (single-precision)"))
  ;[1 1 1] Tank Turret Turn Logic
  (`SceneComponent.K2_AddWorldRotation` (`self.Turret`) (`KismetMathLibrary.MakeRotator` 0.0 0.0 (* AxisValue 2.0)) false false))

(event `InputAxis|MouseLookUp`
  (params (AxisValue :type "Float (single-precision)"))
  ;[1 1 1] Tank Barrel Movement
  (bind _output_get (set `self.CurrentBarrelPitch` (`KismetMathLibrary.FClamp` (+ (`self.CurrentBarrelPitch`) (* AxisValue 2.0)) -90.0 -40.0)))
  (`SceneComponent.K2_SetRelativeRotation` (`self.Barrel`) (`KismetMathLibrary.MakeRotator` 0.0 _output_get) false false))

(event `self.ReceiveBeginPlay`
  ;[1 1 1] Tank Barrel Movement
  (set `self.CurrentBarrelPitch` -90.0))

(event `FireProjectile`
  (bind _projectilespawnpoint (`self.ProjectileSpawnPoint`))
  ;[1 1 1] Firing Logic
  (bind _returnvalue (`|SpawnActorFromClass` "/Game/MathForGames/BP_Projectile.BP_Projectile_C" (`SceneComponent.K2_GetComponentToWorld` _projectilespawnpoint) "Undefined" "MultiplyWithRoot" null null))
  (`PrimitiveComponent.AddImpulse` (`/Game/MathForGames/BP_Projectile.Projectile` _returnvalue) (* (`SceneComponent.GetForwardVector` _projectilespawnpoint) 5000.0) "None" false))

(event `InputAction|Fire`
  (params (Key :type "Key Structure"))
  ;[1 1 1] Firing Logic
  (:`Pressed`
    (`KismetSystemLibrary.K2_SetTimer` null "FireProjectile" 0.2 true true))
  (:`Released`
    (`KismetSystemLibrary.K2_ClearTimer` null "FireProjectile")))

(event `InputAxis|TankZoom`
  (params (AxisValue :type "Float (single-precision)"))
  (bind _camera (`self.Camera`))
  (`CameraComponent.SetFieldOfView` _camera (`KismetMathLibrary.FClamp` (+ (`CameraComponent.FieldOfView` _camera) (* AxisValue 10.0)) 75.0 125.0)))

(event `InputAction|CameraToggle`
  (params (Key :type "Key Structure"))
  (bind _camera (`self.Camera`))
  (bind _topdowncam (`self.TopDownCam`))
  ;[1 1 1] Camera Toggle
  (:`Pressed`
    (bind _output_get (set `self.TopDownActive` (not (`self.TopDownActive`))))
    (if _output_get
      (`ActorComponent.SetActive` _topdowncam true false)
      (`ActorComponent.SetActive` _camera false false)
      (else
        (`ActorComponent.SetActive` _camera true false)
        (`ActorComponent.SetActive` _topdowncam false false)))))

(fn `UserConstructionScript`)