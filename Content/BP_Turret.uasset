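; A turret actor that yaws to face the first player's pawn while it is within detection range.
; Each tick it compares the dot product of its forward vector and the player direction to skip turning when nearly aligned.
; Otherwise the Z sign of their cross product picks the turn direction, applied as a frame-rate independent local rotation at a set speed.
; It contains no firing logic.
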(event `self.ReceiveBeginPlay`
  (set `self.PlayerRef` (`GameplayStatics.GetPlayerPawn` 0)))

(event `self.ReceiveTick`
  (params (DeltaSeconds :type "Float (single-precision)"))
  (bind _returnvalue (`self.GetActorForwardVector`))
  (bind _playerref (`self.PlayerRef`))
  (bind _returnvalue_2 (- (`self.K2_GetActorLocation` _playerref) (`self.K2_GetActorLocation`)))
  (bind _returnvalue_3 (`KismetMathLibrary.Normal` _returnvalue_2))
  (bind (_returnvalue_x _returnvalue_y _returnvalue_z) (`KismetMathLibrary.BreakVector` (`KismetMathLibrary.Cross_VectorVector` _returnvalue _returnvalue_3)))
  (if (`KismetSystemLibrary.IsValid` _playerref)
    (`/Engine/EditorBlueprintResources/StandardMacros.CompareFloat` (`KismetMathLibrary.VSize` _returnvalue_2) (`self.DetectionRange`)
      (:`<`
        (if (> (`KismetMathLibrary.Dot_VectorVector` _returnvalue_3 _returnvalue) 0.99)
          _
          (elif (> _returnvalue_z 0.0)
            (`self.K2_AddActorLocalRotation` (`KismetMathLibrary.MakeRotator` 0.0 0.0 (* (`GameplayStatics.GetWorldDeltaSeconds`) (`self.RotationsSpeed`))))
            (else
              (`self.K2_AddActorLocalRotation` (`KismetMathLibrary.MakeRotator` 0.0 0.0 (* (`GameplayStatics.GetWorldDeltaSeconds`) (`self.RotationsSpeed`) -1.0))))))))))

(fn `UserConstructionScript`)