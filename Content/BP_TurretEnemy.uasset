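; Turret enemy that pops up when the player pawn comes within detection range and retracts when the pawn leaves it.
; Tick compares player distance to the range, toggling an exposed flag and offsetting the Body vertically in while loops that finish within one frame.
; While exposed, it yaws toward the player at a set speed, using a dot product for alignment and cross product Z for turn direction.
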(event `self.ReceiveTick`
  (params (DeltaSeconds :type "Float (single-precision)"))
  (bind _returnvalue (`self.GetActorForwardVector`))
  (bind _playerref (`self.PlayerRef`))
  (bind _body (`self.Body`))
  (bind _turretexpose (`self.TurretExpose`))
  (bind (_relativelocation_x _relativelocation_y _relativelocation_z) (`KismetMathLibrary.BreakVector` (`SceneComponent.RelativeLocation` _body)))
  (bind _returnvalue_2 (- (`self.K2_GetActorLocation` _playerref) (`self.K2_GetActorLocation`)))
  (bind _returnvalue_3 (`KismetMathLibrary.Normal` _returnvalue_2))
  (bind (_returnvalue_x _returnvalue_y _returnvalue_z) (`KismetMathLibrary.BreakVector` (`KismetMathLibrary.Cross_VectorVector` _returnvalue _returnvalue_3)))
  (if (`KismetSystemLibrary.IsValid` _playerref)
    (`/Engine/EditorBlueprintResources/StandardMacros.CompareFloat` (`KismetMathLibrary.VSize` _returnvalue_2) (`self.DetectionRange`)
      (:`>`
        (if _turretexpose :!label _label
          (while (> _relativelocation_z -45.0)
            (`SceneComponent.K2_AddLocalOffset` _body (0.0 0.0 -4.5) false false))
          (set `self.TurretExpose` false)))
      (:`==`
        (goto _label))
      (:`<`
        (if _turretexpose
          (if (> (`KismetMathLibrary.Dot_VectorVector` _returnvalue _returnvalue_3) 0.99)
            _
            (elif (> _returnvalue_z 0.0)
              (`self.K2_AddActorLocalRotation` (`KismetMathLibrary.MakeRotator` 0.0 0.0 (* (`GameplayStatics.GetWorldDeltaSeconds`) (`self.RotationSpeed`))))
              (else
                (`self.K2_AddActorLocalRotation` (`KismetMathLibrary.MakeRotator` 0.0 0.0 (* (`GameplayStatics.GetWorldDeltaSeconds`) (`self.RotationSpeed`) -1.0))))))
          (else
            (while (< _relativelocation_z 90.0)
              (`SceneComponent.K2_AddLocalOffset` _body (0.0 0.0 4.5) false false))
            (set `self.TurretExpose` true)))))))

(event `self.ReceiveBeginPlay`
  (set `self.PlayerRef` (`GameplayStatics.GetPlayerPawn` 0)))

(fn `UserConstructionScript`)