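; BP_Target is a math-prototype target that continuously yaws at a constant, frame-rate-independent speed and reports which side was hit.
; On a component hit, it normalizes the inverted hit normal and takes its dot product with TargetBase's forward vector.
; Thresholds on that result classify the hit as front, back or side, which is shown only through a Print String.
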(event `self.ReceiveTick`
  (params (DeltaSeconds :type "Float (single-precision)"))
  ;[1 1 1] Rotation Logic
  (`SceneComponent.K2_AddLocalRotation` (`self.TargetBase`) (`KismetMathLibrary.MakeRotator` 0.0 0.0 (* (`GameplayStatics.GetWorldDeltaSeconds`) 90.0)) false false))

(event `self.TargetBase.OnComponentHit`
  (params (HitComponent :type "PrimitiveComponent Object Reference") (OtherActor :type "Actor Object Reference") (OtherComp :type "PrimitiveComponent Object Reference") (NormalImpulse :type "Vector Structure") (Hit :type "HitResult Structure (by ref)"))
  (bind _returnvalue (`KismetMathLibrary.Dot_VectorVector` (`KismetMathLibrary.Normal` (* (`.Normal` (`GameplayStatics.BreakHitResult` Hit)) -1.0)) (`SceneComponent.GetForwardVector` (`self.TargetBase`))))
  ;[1 1 1] Target Hit Location (Direction Detection using dot product)
  (if (> _returnvalue 0.5)
    (`KismetSystemLibrary.PrintString` "Front hit!")
    (elif (< _returnvalue -0.5)
      (`KismetSystemLibrary.PrintString` "Back hit!")
      (else
        (`KismetSystemLibrary.PrintString` "Side hit!")))))

(fn `UserConstructionScript`)