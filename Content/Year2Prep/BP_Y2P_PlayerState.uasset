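; Player state Blueprint that keeps the player's score and a time-windowed pickup combo multiplier.
; AddScore updates the combo first, then adds the points times the multiplier and broadcasts the new score.
; UpdateCombo raises the multiplier for pickups within the combo window, otherwise resets it to one, broadcasting either way.
; Each pickup restarts a timer that calls ResetCombo when the window expires.
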(fn `AddScore`
  (params (PointsToAdd :type Integer))
  (`self.UpdateCombo`)
  (bind _output_get (set `self.MyScore` (+ (* PointsToAdd (`self.ComboMultiplier`)) (`self.MyScore`))))
  (`self.OnScoreChanged` _output_get))

(fn `ResetCombo`
  (bind _output_get (set `self.ComboMultiplier` 1))
  (`self.OnComboChanged` _output_get))

(fn `UpdateCombo`
  (bind _returnvalue (`KismetSystemLibrary.GetGameTimeInSeconds`))
  (if (< (- _returnvalue (`self.LastPickupTime`)) (`self.ComboWindow`))
    (bind _result (`/Engine/EditorBlueprintResources/StandardMacros.IncrementInt` (`self.ComboMultiplier`))
      (:`  `
        (`self.OnComboChanged` _result)))
    (else
      (set `self.ComboMultiplier` 1)
      (`self.OnComboChanged` 1)))
  (set `self.LastPickupTime` _returnvalue)
  (`KismetSystemLibrary.K2_ClearAndInvalidateTimerHandle` (`self.ComboResetTimer`))
  (bind _returnvalue_2 (`KismetSystemLibrary.K2_SetTimer` null "ResetCombo" (`self.ComboWindow`)))
  (set `self.ComboResetTimer` _returnvalue_2))

(fn `UserConstructionScript`)