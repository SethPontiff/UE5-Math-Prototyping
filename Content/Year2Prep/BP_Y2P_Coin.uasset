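; Collectible coin that adds its Points to the Y2P player state's score when a Y2P character overlaps it, then destroys itself.
; Tick spins the coin mesh around Z, and the construction script feeds StartPoint and EndPoint to an InterpToMovement component as relative control points.
; A self-rescheduling ToggleVisibility timer function alternates visibility and collision, but its starting call is disconnected, as is older collection logic for other player classes.
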(event `self.ReceiveTick`
  (params (DeltaSeconds :type "Float (single-precision)"))
  ;[1 1 1] Rotation Logic
  (`SceneComponent.K2_AddRelativeRotation` (`self.Coin`) (`KismetMathLibrary.RotatorFromAxisAndAngle` (0.0 0.0 1.0) (* (`self.RotationSpeed`) (`GameplayStatics.GetWorldDeltaSeconds`))) false false))

(event `self.ReceiveBeginPlay`
  ;[1 1 1] Vanishing
)

(event `self.ReceiveActorBeginOverlap`
  (params (OtherActor :type "Actor Object Reference"))
  (bind _asbp_y2p_character (cast `/Game/Year2Prep/BP_Y2P_Character` OtherActor))
  (bind _asbp_y2p_player_state (cast `/Game/Year2Prep/BP_Y2P_PlayerState` (`Pawn.PlayerState` _asbp_y2p_character)))
  (`/Game/Year2Prep/BP_Y2P_PlayerState.AddScore` _asbp_y2p_player_state (`self.Points`))
  (`self.K2_DestroyActor`))

(fn `ToggleVisibility`
  (bind _output_get (set `self.IsVisible` (not (`self.IsVisible`))))
  (if _output_get
    (`self.SetActorHiddenInGame` false)
    (`self.SetActorEnableCollision` true)
    (`KismetSystemLibrary.K2_SetTimer` null "ToggleVisibility" (`self.AppearDuration`))
    (else
      (`self.SetActorHiddenInGame` true)
      (`self.SetActorEnableCollision` false)
      (`KismetSystemLibrary.K2_SetTimer` null "ToggleVisibility" (`self.DisappearDuration`)))))

(fn `UserConstructionScript`
  (`InterpToMovementComponent.AddControlPointPosition` (`self.InterpToMovement`) (`self.StartPoint`) true)
  (`InterpToMovementComponent.AddControlPointPosition` (`self.InterpToMovement`) (`self.EndPoint`) true))