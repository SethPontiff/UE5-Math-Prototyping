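; BP_GES_PlayerState is a player state Blueprint that holds the player's points and exposes functions to add and read them.
; AddPoints reassigns CurrentPoints to itself without using PointsToAdd, then casts through the owning PlayerController to BP_GES_HUD to refresh the PlayerHUD points display.
; GetPoints returns CurrentPoints.
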(fn `AddPoints`
  (params (PointsToAdd :type Integer))
  (set `self.CurrentPoints` (`self.CurrentPoints`))
  (bind _asplayer_controller (cast `PlayerController` (`self.GetOwner`)))
  (bind _asbp_ges_hud (cast `/Game/GameEngineScripting/Widgets/BP_GES_HUD` (`PlayerController.GetHUD` _asplayer_controller)))
  (`/Game/GameEngineScripting/Widgets/WBP_GES_PlayerHUD.UpdatePointsDisplay` (`/Game/GameEngineScripting/Widgets/BP_GES_HUD.PlayerHUD` _asbp_ges_hud)))

(fn `GetPoints`
  (returns (ReturnValue :type Integer))
  (return (`self.CurrentPoints`)))

(fn `UserConstructionScript`)