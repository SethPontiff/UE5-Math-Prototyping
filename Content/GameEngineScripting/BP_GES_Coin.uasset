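; BP_GES_Coin is a collectible coin that spins, moves between two points and periodically vanishes.
; The construction script feeds StartPoint and EndPoint to InterpToMovement as relative control points, while Tick rotates the Coin component.
; A self-rescheduling ToggleVisibility timer alternates visibility and collision using separate appear and disappear durations.
; Overlap by BP_ThirdPersonCharacter adds Points to BP_GES_PlayerState, destroys the coin and prints the total.
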(event `self.ReceiveTick`
  (params (DeltaSeconds :type "Float (single-precision)"))
  ;[1 1 1] Rotation Logic
  (`|ExecutionSequence`
    (:`then_1`
      (`SceneComponent.K2_AddRelativeRotation` (`self.Coin`) (`KismetMathLibrary.RotatorFromAxisAndAngle` (0.0 0.0 1.0) (* (`self.RotationSpeed`) (`GameplayStatics.GetWorldDeltaSeconds`))) false false))))

(event `self.ReceiveBeginPlay`
  ;[1 1 1] Moving Coin
  (`|ExecutionSequence`
    (:`then_0`
      (bind _output_get (set `self.InitialLocation` (`self.K2_GetActorLocation`)))
      (set `self.CurrentTarget` (+ _output_get (`self.EndPoint`))))
    (:`then_1`
      ;[1 1 1] Vanishing
      (`KismetSystemLibrary.K2_SetTimer` null "ToggleVisibility" (`self.AppearDuration`)))))

(event `self.ReceiveActorBeginOverlap`
  (params (OtherActor :type "Actor Object Reference"))
  ;[1 1 1] Pickup Destruction
  ;[1 1 1] Coin Collection & Update
  (bind _asbp_third_person_character (cast `/Game/ThirdPerson/Blueprints/BP_ThirdPersonCharacter` OtherActor))
  (bind _asbp_ges_player_state (cast `/Game/GameEngineScripting/BP_GES_PlayerState` (`Pawn.PlayerState` _asbp_third_person_character)))
  (bind _currentpoints (`/Game/GameEngineScripting/BP_GES_PlayerState.CurrentPoints` _asbp_ges_player_state))
  (set `/Game/GameEngineScripting/BP_GES_PlayerState.CurrentPoints` (+ (`self.Points`) _currentpoints) _asbp_ges_player_state)
  (`self.K2_DestroyActor`)
  (`KismetSystemLibrary.PrintString` (`KismetStringLibrary.Conv_IntToString` _currentpoints)))

(fn `ToggleVisibility`
  (bind _output_get (set `self.IsVisible` (not (`self.IsVisible`))))
  (if _output_get
    (`self.SetActorHiddenInGame` false)
    (`self.SetActorEnableCollision` true)
    (`KismetSystemLibrary.K2_SetTimer` null "ToggleVisibility" (`self.AppearDuration`))
    (else
      (`self.SetActorHiddenInGame` true)
      (`self.SetActorEnableCollision` false)
      (`KismetSystemLibrary.K2_SetTimer` null "ToggleVisibility" (`self.DisappearDuration`)))))

(fn `UserConstructionScript`
  (`InterpToMovementComponent.AddControlPointPosition` (`self.InterpToMovement`) (`self.StartPoint`) true)
  (`InterpToMovementComponent.AddControlPointPosition` (`self.InterpToMovement`) (`self.EndPoint`) true))