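; Player character that picks a class through a selection widget and swings a class-specific melee weapon.
; BeginPlay adds the Enhanced Input mapping for move, look, jump and attack, then shows the class selection UI in UI-only input mode.
; LoadClass, not called within this Blueprint, spawns the class data's primary weapon and snaps it to WeaponAttachmentPoint.
; Attack rotates that attachment point with a curve timeline, blocking new swings until it finishes.
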(event `self.ReceiveBeginPlay`
  ;[1 1 1] Grabbing Input Mapping At Start
  (`|ExecutionSequence`
    (:`then_0`
      (bind _asplayer_controller (cast `PlayerController` (`self.GetController`)))
      (bind _returnvalue (pcsubsystem `EnhancedInputLocalPlayerSubsystem` _asplayer_controller))
      (`/Engine/EditorBlueprintResources/StandardMacros.IsValid` _returnvalue
        (:`Is Valid`
          (`EnhancedInputSubsystemInterface.AddMappingContext` _returnvalue "/Game/GameEngineScripting/Inputs/IMC_GES_Default.IMC_GES_Default" 0 (struct)))))
    (:`then_1`
      (bind _returnvalue_2 (`|CreateWidget` "/Game/GameEngineScripting/WBP_ClassSelection.WBP_ClassSelection_C"))
      (`UserWidget.AddToViewport` _returnvalue_2 0)
      (`WidgetBlueprintLibrary.SetInputMode_UIOnlyEx` _asplayer_controller null)
      (set `PlayerController.bShowMouseCursor` true _asplayer_controller))))

(event `EnhancedInput|/Game/GameEngineScripting/Inputs/IA_GES_Jump`
  (params (ActionValue :type Boolean) (ElapsedSeconds :type "Float (double-precision)") (TriggeredSeconds :type "Float (double-precision)") (InputAction :type "InputAction Object Reference" :default "/Game/GameEngineScripting/Inputs/IA_GES_Jump.IA_GES_Jump"))
  ;[1 1 1] Jumping Logic
  (:`Triggered`
    (`self.Jump`))
  (:`Completed`
    (`self.StopJumping`)))

(event `EnhancedInput|/Game/GameEngineScripting/Inputs/IA_GES_Look`
  (params (ActionValue :type "Vector2D Structure") (ElapsedSeconds :type "Float (double-precision)") (TriggeredSeconds :type "Float (double-precision)") (InputAction :type "InputAction Object Reference" :default "/Game/GameEngineScripting/Inputs/IA_GES_Look.IA_GES_Look"))
  ;[1 1 1] Camera
  (:`Triggered`
    (`self.AddControllerYawInput` ActionValue_X)
    (`self.AddControllerPitchInput` ActionValue_Y)))

(event `EnhancedInput|/Game/GameEngineScripting/Inputs/IA_GES_Move`
  (params (ActionValue :type "Vector2D Structure") (ElapsedSeconds :type "Float (double-precision)") (TriggeredSeconds :type "Float (double-precision)") (InputAction :type "InputAction Object Reference" :default "/Game/GameEngineScripting/Inputs/IA_GES_Move.IA_GES_Move"))
  (bind (_returnvalue_roll _returnvalue_pitch _returnvalue_yaw) (`KismetMathLibrary.BreakRotator` (`self.GetControlRotation`)))
  (bind (_returnvalue_roll_2 _returnvalue_pitch_2 _returnvalue_yaw_2) (`KismetMathLibrary.BreakRotator` (`self.GetControlRotation`)))
  ;[1 1 1] Movement Inputs
  (:`Triggered`
    (`self.AddMovementInput` (`KismetMathLibrary.GetRightVector` (`KismetMathLibrary.MakeRotator` _returnvalue_roll_2 0.0 _returnvalue_yaw_2)) ActionValue_X)
    (`self.AddMovementInput` (`KismetMathLibrary.GetForwardVector` (`KismetMathLibrary.MakeRotator` 0.0 0.0 _returnvalue_yaw)) ActionValue_Y)))

(event `EnhancedInput|/Game/GameEngineScripting/Inputs/IA_GES_Attack`
  (params (ActionValue :type Boolean) (ElapsedSeconds :type "Float (double-precision)") (TriggeredSeconds :type "Float (double-precision)") (InputAction :type "InputAction Object Reference" :default "/Game/GameEngineScripting/Inputs/IA_GES_Attack.IA_GES_Attack"))
  ;[1 1 1] Weapon Attack
  (:`Triggered`
    (if (not (`self.SwingOnCooldown`))
      (set `self.SwingOnCooldown` true)
      (bind (_direction _swingcurve) (`Timeline|WeaponSwing` :!via `PlayFromStart`)
        (:`Update`
          (`SceneComponent.K2_SetRelativeRotation` (`self.WeaponAttachmentPoint`) (`KismetMathLibrary.RLerp` (struct) (struct :`Pitch` -90.0) _swingcurve) false false))
        (:`Finished`
          (set `self.SwingOnCooldown` false))))))

(fn `LoadClass`
  (params (ClassData :type "/Game/GameEngineScripting/DataAssets/BP_GES_ClassData Object Reference"))
  (bind _returnvalue (`|SpawnActorFromClass` (`/Game/GameEngineScripting/DataAssets/BP_GES_ClassData.PrimaryWeaponMesh` ClassData) (`self.GetTransform`) "Undefined" "MultiplyWithRoot" null null))
  (`self.K2_AttachToComponent` _returnvalue (`self.WeaponAttachmentPoint`) "None" "SnapToTarget" "SnapToTarget" "SnapToTarget" true))

(fn `UserConstructionScript`)