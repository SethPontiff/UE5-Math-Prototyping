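; BP_AutoTurret is a turret actor that turns to face the player while they are within DetectionRange.
; It caches the player pawn on BeginPlay and checks its distance every Tick.
; A dot product detects when the turret is nearly aligned and prints a debug message; otherwise the cross product's Z sign picks the yaw direction, turning at RotationSpeed scaled by delta time.
; It has no firing logic.
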(event `self.ReceiveBeginPlay`
  (set `self.PlayerRef` (`GameplayStatics.GetPlayerPawn` 0)))

(event `self.ReceiveTick`
  (params (DeltaSeconds :type "Float (single-precision)"))
  (bind _returnvalue (`self.GetActorForwardVector`))
  (bind _playerref (`self.PlayerRef`))
  (bind _returnvalue_2 (- (`self.K2_GetActorLocation` _playerref) (`self.K2_GetActorLocation`)))
  (bind _returnvalue_3 (`KismetMathLibrary.Normal` _returnvalue_2))
  (if (`KismetSystemLibrary.IsValid` _playerref)
    (`/Engine/EditorBlueprintResources/StandardMacros.CompareFloat` (`KismetMathLibrary.VSize` _returnvalue_2) (`self.DetectionRange`)
      (:`<`
        (if true
          (if (> (`KismetMathLibrary.Dot_VectorVector` _returnvalue _returnvalue_3) 0.99)
            (`KismetSystemLibrary.PrintString` "In Front of Player")
            (elif (> (.z (`KismetMathLibrary.Cross_VectorVector` _returnvalue _returnvalue_3)) 0.0)
              (`self.K2_AddActorLocalRotation` (`KismetMathLibrary.MakeRotator` 0.0 0.0 (* (`GameplayStatics.GetWorldDeltaSeconds`) (`self.RotationSpeed`))))
              (else
                (`self.K2_AddActorLocalRotation` (`KismetMathLibrary.MakeRotator` 0.0 0.0 (* (* (`GameplayStatics.GetWorldDeltaSeconds`) (`self.RotationSpeed`)) -1.0)))))))))))

(fn `UserConstructionScript`)